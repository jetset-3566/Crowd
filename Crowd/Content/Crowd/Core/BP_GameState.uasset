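; Game state for the crowd system that registers spawn points and relays group-level commands to their bots.
; Bots are looked up through the spawn points by setting name, with "None" selecting every group.
; Events press all spawn points, send a group a charge message that changes chase state, or toggle target and debug displays through the CRW_IBot interface.
; Helpers report group names and bot counts, while AddAiActor is an empty stub.
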(event `AddSpawnPoint`
  (params (newPoint :type "/Game/Crowd/Core/AISpawn/SpawnPoint/BP_SpawnPointStart Object Reference"))
  (`KismetArrayLibrary.Array_Add` (`self.SpawnPoints`) newPoint))

(event `AddAiActor`
  (params (newBot :type "Actor Object Reference") (Name :type "Name (by ref)")))

(event `PessedAllSpawnPoint`
  (for _array_element (`self.SpawnPoints`)
    (`/Game/Crowd/Core/AISpawn/SpawnPoint/BP_SpawnPointStart.OnPressed` _array_element)))

(event `StartCharge`
  (params (Group :type Name))
  (bind _bots (`self.GetBotsRefByGroup` Group))
  (for _array_element _bots
    (message `CRW_IBot.ChangeChaseStateCurrentTarget` _array_element)))

(event `ShowDebugByGroupAndCommand`
  (params (Group :type "Name (by ref)") (DebugCommand :type Name) (bIsOn :type Boolean))
  (bind _bots (`self.GetBotsRefByGroup` Group))
  (`self.ShowHideDebug` _bots DebugCommand bIsOn))

(fn `GetBotsCoutByGroup`
  (params (Name :type Name))
  (returns (Cout :type Integer))
  (locals (BotsCouts :type Integer :default 0))
  (for _array_element (`self.SpawnPoints`)
    (if (== (`.Name` (break `SpawnSetting` (`/Game/Crowd/Core/AISpawn/SpawnPoint/BP_SpawnPointStart.SpawnSetting` _array_element))) Name)
      (set `local.BotsCouts` (`KismetArrayLibrary.Array_Length` (`/Game/Crowd/Core/AISpawn/SpawnPoint/BP_SpawnPointStart.Bots` _array_element)))
      (break)))
  (return (`local.BotsCouts`)))

(fn `GetBotsRefByGroup`
  (params (Group :type Name))
  (returns (Bots :type "Array of Actor Object Reference"))
  (locals (Current :type "Array of Actor Object Reference"))
  (bind _current (`local.Current`))
  (bind _spawnpoints (`self.SpawnPoints`))
  (bind _current_2 (`local.Current`))
  (if (== Group "None")
    (for _array_element _spawnpoints
      (`KismetArrayLibrary.Array_Append` _current_2 (`/Game/Crowd/Core/AISpawn/SpawnPoint/BP_SpawnPointStart.Bots` _array_element)))
    (return _current_2)
    (else
      (for _array_element_2 _spawnpoints
        (if (== (`.Name` (break `SpawnSetting` (`/Game/Crowd/Core/AISpawn/SpawnPoint/BP_SpawnPointStart.SpawnSetting` _array_element_2))) Group)
          (`KismetArrayLibrary.Array_Append` _current (`/Game/Crowd/Core/AISpawn/SpawnPoint/BP_SpawnPointStart.Bots` _array_element_2))))
      (return _current))))

(fn `GetGroupsOfMap`
  (returns (Name :type "Array of Name"))
  (locals (Names :type "Array of Name"))
  (bind _names (`local.Names`))
  (for _array_element (`self.SpawnPoints`)
    (`KismetArrayLibrary.Array_Add` _names (`.Name` (break `SpawnSetting` (`/Game/Crowd/Core/AISpawn/SpawnPoint/BP_SpawnPointStart.SpawnSetting` _array_element)))))
  (return _names))

(fn `ShowHideDebug`
  (params (Actors :type "Array of Actor Object Reference") (DebugCommand :type Name) (IsOn :type Boolean))
  (for _array_element Actors
    (bind _ascrw_ibot (cast `CRW_IBot` _array_element))
    (switch `name` DebugCommand
      (:`Default`
        (`KismetSystemLibrary.PrintString` "Error: BP_GameState_ShowHideDebug() - Not Have this Command" true true (struct :`R` 1.0 :`B` 0.208042 :`A` 1.0)))
      (:`ShowTarget`
        (`CRW_IBot.ShowTargetPoint` _ascrw_ibot IsOn))
      (:`ShowDebug`
        (`CRW_IBot.ShowDebugInfo` _ascrw_ibot IsOn)))))

(fn `UserConstructionScript`)