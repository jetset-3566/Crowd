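; Debug helper component for crowd bots that shows an info label and target arrows on its owner.
; On BeginPlay it adds a hidden screen-space BPW_InfoUnit widget; info updates set its text and tint the static mesh by helper index.
; A BotState bitmask holds the debug and chase flags, toggled by events.
; Tick reads it to draw an arrow to the current target, colored by chase state, or upward without one.
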(event `self.UpdateCommonInfo`
  (bind _widgetinfo (`self.WidgetInfo`))
  (`/Engine/EditorBlueprintResources/StandardMacros.IsValid` _widgetinfo
    (:`Is Valid`
      (bind _asbpw_info_unit (cast `/Game/Crowd/Core/AISpawn/HelperUnitWidget/BPW_InfoUnit` (`WidgetComponent.GetUserWidgetObject` _widgetinfo)))
      (`/Game/Crowd/Core/AISpawn/HelperUnitWidget/BPW_InfoUnit.SetText` _asbpw_info_unit (`self.Info`))
      (`self.UpdateColorTypeOfOwner`))))

(event `self.StartChaseCurrentTarget`
  (bind _botstate (`self.BotState`))
  (`/Engine/EditorBlueprintResources/StandardMacros.IsValid` (`self.GetCurrentTarget`)
    (:`Is Valid`
      (`CRW_CommonLibrary.SetFlagBotStateByByte` _botstate 2 (not (`CRW_CommonLibrary.BotStateCheckByByte` _botstate 2))))))

(event `self.ReceiveBeginPlay`
  (`self.AddWidgetComponetToOwner`))

(event `self.ShowDebugInfo`
  (params (bIsShow :type Boolean))
  (`SceneComponent.SetVisibility` (`self.WidgetInfo`) bIsShow false))

(event `self.ShowTargetPoint`
  (params (bIsShow :type Boolean))
  (`CRW_CommonLibrary.SetFlagBotStateByByte` (`self.BotState`) 1 bIsShow))

(event `self.ReceiveTick`
  (params (DeltaSeconds :type "Float (single-precision)"))
  (bind _returnvalue (`self.GetCurrentTarget`))
  (bind _botstate (`self.BotState`))
  (bind _returnvalue_2 (`Actor.K2_GetActorLocation` (`self.GetOwner`)))
  (bind _returnvalue_3 (+ _returnvalue_2 (0.0 0.0 100.0)))
  (`|ExecutionSequence`
    (:`then_0`
      (if (`CRW_CommonLibrary.BotStateCheckByByte` _botstate 1)
        (`/Engine/EditorBlueprintResources/StandardMacros.IsValid` _returnvalue
          (:`Is Valid`
            (`KismetSystemLibrary.DrawDebugArrow` _returnvalue_3 (+ (`Actor.K2_GetActorLocation` _returnvalue) (0.0 0.0 100.0)) 10.0 (select `bool` (`CRW_CommonLibrary.BotStateCheckByByte` _botstate 2) :`false` (struct :`R` 1.0 :`A` 1.0) :`true` (struct :`R` 0.010704 :`G` 1.0 :`A` 1.0) :!type "LinearColor Structure") 0.0 5.0))
          (:`Is Not Valid`
            (`KismetSystemLibrary.DrawDebugArrow` _returnvalue_2 _returnvalue_3 10.0 (struct) 0.0 5.0)))))))

(fn `AddWidgetComponetToOwner`
  (bind _returnvalue (`self.GetOwner`))
  (bind _widgetinfo (`self.WidgetInfo`))
  (bind _returnvalue_2 (`|AddComponentByClass` _returnvalue "/Script/UMG.WidgetComponent" false (`KismetMathLibrary.MakeTransform` (0.0 0.0 0.0))))
  (set `self.WidgetInfo` _returnvalue_2)
  (`WidgetComponent.SetWidgetSpace` _widgetinfo "Screen")
  (`WidgetComponent.SetDrawAtDesiredSize` _widgetinfo true)
  (bind _returnvalue_3 (`|CreateWidget` "/Game/Crowd/Core/AISpawn/HelperUnitWidget/BPW_InfoUnit.BPW_InfoUnit_C" null "None"))
  (`WidgetComponent.SetWidget` _widgetinfo _returnvalue_3)
  (`SceneComponent.K2_AttachToComponent` _widgetinfo (`Actor.RootComponent` _returnvalue) "Head" "KeepRelative" "KeepRelative" "KeepRelative" true)
  (`SceneComponent.K2_AddRelativeLocation` _widgetinfo (0.0 0.0 100.0) false false)
  (`SceneComponent.SetVisibility` _widgetinfo false false))

(fn `UpdateColorTypeOfOwner`
  (locals (Colors :type "Array of LinearColor Structure"))
  (bind _returnvalue (`self.GetOwner`))
  (bind _colors (`local.Colors`))
  (bind _currenthelperindex (`self.CurrentHelperIndex`))
  (bind _returnvalue_2 (`Actor.GetComponentByClass` _returnvalue "/Script/Engine.StaticMeshComponent"))
  (bind _returnvalue_3 (`KismetMathLibrary.MakeRandomStream` _currenthelperindex))
  (bind _returnvalue_4 (`KismetMathLibrary.MakeRandomStream` (+ _currenthelperindex 10)))
  (`/Engine/EditorBlueprintResources/StandardMacros.IsValid` _returnvalue_2
    (:`Is Valid`
      (bind _returnvalue_5 (`PrimitiveComponent.CreateDynamicMaterialInstance` _returnvalue_2 0 (`PrimitiveComponent.GetMaterial` _returnvalue_2 0) "None"))
      (`MaterialInstanceDynamic.SetVectorParameterValue` _returnvalue_5 "BaseColor" (`KismetMathLibrary.SelectColor` (`|GetArrayItem` _colors (- _currenthelperindex 1)) (`KismetMathLibrary.MakeColor` (`KismetMathLibrary.RandomFloatInRangeFromStream` 0.5 1.0 _returnvalue_4) (`KismetMathLibrary.RandomFloatInRangeFromStream` 0.5 1.0 _returnvalue_4) (`KismetMathLibrary.RandomFloatInRangeFromStream` 0.5 1.0 _returnvalue_4)) (`KismetArrayLibrary.Array_IsValidIndex` _colors _currenthelperindex)))
      (`MaterialInstanceDynamic.SetVectorParameterValue` _returnvalue_5 "SecondColor" (make `LinearColor` (`KismetMathLibrary.RandomFloatInRangeFromStream` 0.5 4.0 _returnvalue_3) (`KismetMathLibrary.RandomFloatInRangeFromStream` 0.5 4.0 _returnvalue_3) (`KismetMathLibrary.RandomFloatInRangeFromStream` 0.5 4.0 _returnvalue_3) 1.0))
      (`PrimitiveComponent.SetMaterial` _returnvalue_2 0 _returnvalue_5))
    (:`Is Not Valid`
      (`/Engine/EditorBlueprintResources/StandardMacros.IsValid` (`Actor.GetComponentByClass` _returnvalue "/Script/Engine.SkeletalMeshComponent")
        (:`Is Not Valid`
          (`KismetSystemLibrary.PrintString` "BP_HelperBotComponent::UpdateColorTypeOfOnwer Not Find Any mesh in owner of actor"))))))