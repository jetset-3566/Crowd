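; AI actor with a UFO mesh that chases its current target using physics-driven movement.
; Each Tick, while BPHelperBotComponent reports the chasing state with a valid target, it checks whether the target lies beyond a distance tolerance.
; If so, dot products against right and forward vectors pick the yaw torque direction and forward or reverse force, both applied to the mesh as acceleration changes.
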(event `self.ReceiveTick`
  (params (DeltaSeconds :type "Float (single-precision)"))
  (bind _bp_helperbotcomponent (`self.BP_HelperBotComponent`))
  (bind _result (`/Game/Crowd/Core/BP_HelperBotComponent.CheckStateByEnum` _bp_helperbotcomponent "IsChasing"))
  (if _result
    (`/Engine/EditorBlueprintResources/StandardMacros.IsValid` (`CRW_HelperBot.GetCurrentTarget` _bp_helperbotcomponent)
      (:`Is Valid`
        (bind _indestinatation (`self.FindVectorToTarget`))
        ;[1 1 1] Simple movement
        (if (not _indestinatation)
          (`|ExecutionSequence`
            (:`then_0`
              (bind (_bisright _bisoppositiveturn) (`self.CheckTargetIsRight`))
              (set `self.bIsTurnRight?` _bisright)
              (set `self.bIsUseForceForMovement` _bisoppositiveturn))
            (:`then_1`
              (`PrimitiveComponent.AddForce` (`self.SM_UFO`) (* (`self.GetActorForwardVector`) (* (select `bool` (`self.bIsUseForceForMovement`) :`false` -1.0 :`true` 1.0 :!type "Float (single-precision)") (`self.CoefForceAdd`))) "None" true)
              (`PrimitiveComponent.AddTorqueInRadians` (`self.SM_UFO`) (* (0.0 0.0 1.0) (`KismetMathLibrary.SelectFloat` 1.0 -1.0 (`self.bIsTurnRight?`))) "None" true))))))))

(fn `CheckTargetIsRight`
  (returns (bIsRight :type Boolean) (bIsOppositiveTurn :type Boolean))
  (bind _vectortotarget (`self.VectorToTarget`))
  (return (> (`KismetMathLibrary.Dot_VectorVector` _vectortotarget (`SceneComponent.GetRightVector` (`self.SM_UFO`))) 0.0) (> (`KismetMathLibrary.Dot_VectorVector` _vectortotarget (`self.GetActorForwardVector`)) 0.0)))

(fn `FindVectorToTarget`
  (returns (InDestinatation :type Boolean))
  (bind _returnvalue (- (`self.K2_GetActorLocation` (`CRW_HelperBot.GetCurrentTarget` (`self.BP_HelperBotComponent`))) (`self.K2_GetActorLocation`)))
  (set `self.VectorToTarget` (`KismetMathLibrary.Normal` _returnvalue))
  (return (< (`KismetMathLibrary.VSize` _returnvalue) (`self.ToleranceToDestination`))))

(fn `GetCommonInfo`
  (returns (ReturnValue :type Text))
  (return ""))

(fn `UserConstructionScript`)