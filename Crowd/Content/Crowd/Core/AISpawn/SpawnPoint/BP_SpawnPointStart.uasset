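; Interactable crowd spawn point that registers with BP_GameState on BeginPlay and spawns a group of AI bots when pressed.
; SpawnUnits lays units out in a grid to the left or right, then gives each a name and chase target via CRW_IBot.
; Pressing locks the point until immediate reset, a timer, or destruction of all its bots, depending on TypeOfAviable.
; Material swaps show hovered, pressed and idle states.
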(event `self.ReceiveBeginPlay`
  (bind _asbp_game_state (cast `/Game/Crowd/Core/BP_GameState` (`GameplayStatics.GetGameState`)))
  (bind _output_get (set `self.As BP Game State` _asbp_game_state))
  (`/Game/Crowd/Core/BP_GameState.AddSpawnPoint` _output_get self))

(fn `IsOnHovered`
  (params (bIsHovered :type Boolean))
  (if (`self.bIsAviableForInteract`)
    (`PrimitiveComponent.SetMaterial` (`self.StaticMesh1`) 0 (select `bool` bIsHovered :`false` "/Game/Crowd/Core/AISpawn/SpawnPoint/Material/M_InteractableMateria_NotHoveredl_Inst.M_InteractableMateria_NotHoveredl_Inst" :`true` "/Game/Crowd/Core/AISpawn/SpawnPoint/Material/M_InteractableMaterial_Hovered_Inst1.M_InteractableMaterial_Hovered_Inst1" :!type "MaterialInterface Object Reference"))))

(fn `OnPressed`
  (if (`self.bIsAviableForInteract`)
    (`self.SpawnUnits`)
    (`PrimitiveComponent.SetMaterial` (`self.StaticMesh1`) 0 "/Game/Crowd/Core/AISpawn/SpawnPoint/Material/M_InteractableMaterial_OnPressed_Inst2.M_InteractableMaterial_OnPressed_Inst2")
    (set `self.bIsAviableForInteract` false)
    (switch `/Game/Crowd/Core/AISpawn/SpawnPoint/E_AviableSpawnPoint` (`self.TypeOfAviable`)
      (:`NewEnumerator0`
        (`self.SpawnCoolDownEnd`))
      (:`NewEnumerator1`
        (`KismetSystemLibrary.K2_SetTimer` null "SpawnCoolDownEnd" (`self.TimerAfterPressedButton`)))
      (:`NewEnumerator2`))))

(fn `OnSpawnedActorDestroed`
  (params (DestroyedActor :type "Actor Object Reference"))
  (bind _bots (`self.Bots`))
  (`KismetArrayLibrary.Array_RemoveItem` _bots DestroyedActor)
  (if (<= (`KismetArrayLibrary.Array_Length` _bots) 0)
    (if (`|EnumEquality` (`self.TypeOfAviable`) "NewEnumerator2")
      (`self.SpawnCoolDownEnd`))))

(fn `SpawnCoolDownEnd`
  (set `self.bIsAviableForInteract` true)
  (`self.IsOnHovered` false))

(fn `SpawnUnits`
  (locals (Condition :type Boolean :default true) (CurrentNumbersOfUnitsToSpawn :type Integer) (Row :type Integer))
  (bind _row (`local.Row`))
  (bind _currentnumbersofunitstospawn (`local.CurrentNumbersOfUnitsToSpawn`))
  (bind ((`Name_21_E0F8124F4C7D7C400C726793A3992AF6` _name) (`NumberOfUnit_6_9FD0AB9743CD292FD24C578E66F3ECBE` _numberofunit) (`TargetOfChase_17_94E1842F4E74A3D168F9078D50B398F2` _targetofchase)) (break `/Game/Crowd/Core/AISpawn/SpawnPoint/ST_SpawnSetting` (`self.SpawnSetting`)))
  (bind (_name_2 _class _numberofunit_2 _numberofrow _bisspawntoright) (break `/Game/Crowd/Core/AISpawn/SpawnPoint/ST_SpawnSetting` (`self.SpawnSetting`)))
  (while (`local.Condition`)
    (for _index (range (/ _numberofunit_2 _numberofrow))
      (bind _returnvalue (`|SpawnActorFromClass` _class (`KismetMathLibrary.MakeTransform` (`KismetMathLibrary.MakeVector` (+ (.x (+ (`self.K2_GetActorLocation` self) (`KismetMathLibrary.MakeVector` (select `bool` _bisspawntoright :`false` 200.0 :`true` -200.0 :!type "Float (single-precision)") 0.0 100.0))) (* (* _index 200.0) (select `bool` _bisspawntoright :`false` 1.0 :`true` -1.0 :!type "Float (single-precision)"))) (+ (.y (+ (`self.K2_GetActorLocation` self) (`KismetMathLibrary.MakeVector` (select `bool` _bisspawntoright :`false` 200.0 :`true` -200.0 :!type "Float (single-precision)") 0.0 100.0))) (* _row 200.0)) (.z (+ (`self.K2_GetActorLocation` self) (`KismetMathLibrary.MakeVector` (select `bool` _bisspawntoright :`false` 200.0 :`true` -200.0 :!type "Float (single-precision)") 0.0 100.0))))) "AlwaysSpawn" "OverrideRootScale" null null))
      (add `self.OnDestroyed` _returnvalue (`|CreateDelegate` :!event `OnSpawnedActorDestroed`))
      (bind _ascrw_ibot (cast `CRW_IBot` _returnvalue))
      (`CRW_IBot.SetCommonInfo` _ascrw_ibot (`|FormatText` "{Name} - {I} \n{R}:{C}" _name_2 (+ (`local.CurrentNumbersOfUnitsToSpawn`) 1) _row _index))
      (`CRW_IBot.SetChaseTarget` _ascrw_ibot _targetofchase)
      (`KismetArrayLibrary.Array_Add` (`self.Bots`) _returnvalue)
      (`/Game/Crowd/Core/BP_GameState.AddAiActor` (`self.As BP Game State`) _returnvalue _name) ; not used
      (`/Engine/EditorBlueprintResources/StandardMacros.IncrementInt` _currentnumbersofunitstospawn
        (:`  `
          (bind _output_get (set `local.Condition` (not (>= _currentnumbersofunitstospawn _numberofunit))))
          (if (not _output_get)
            (break)))))
    (`/Engine/EditorBlueprintResources/StandardMacros.IncrementInt` (`local.Row`))))

(fn `UserConstructionScript`)