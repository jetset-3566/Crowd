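; Player controller for a crowd demo that lets the player hover and click spawn points, trigger spawns and group charges, and toggle debugging tools.
; Each tick it traces under the visible cursor to update spawn point hover state and the click target.
; Charge, spawn-all and per-group debug inputs route through BP_GameState.
; Other keys toggle help and animation budget widgets, switch the Animation Budget Allocator, and enable Detour crowd debug drawing via console commands.
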(event `InputAction|ShowTarget`
  (params (Key :type "Key Structure"))
  (bind _gamestate_ref (`self.GameState_ref`))
  (bind _currentgroup (`self.CurrentGroup`))
  ;[1 0.9582 0] Input
  (:`Pressed`
    (`/Game/Crowd/Core/BP_GameState.ShowDebugByGroupAndCommand` _gamestate_ref _currentgroup "ShowTarget" true))
  (:`Released`
    (`/Game/Crowd/Core/BP_GameState.ShowDebugByGroupAndCommand` _gamestate_ref _currentgroup "ShowTarget" false)))

(event `InputAction|ShowDebug`
  (params (Key :type "Key Structure"))
  (bind _gamestate_ref (`self.GameState_ref`))
  (bind _currentgroup (`self.CurrentGroup`))
  ;[1 0.9582 0] Input
  (:`Pressed`
    (`/Game/Crowd/Core/BP_GameState.ShowDebugByGroupAndCommand` _gamestate_ref _currentgroup "ShowDebug" true))
  (:`Released`
    (`/Game/Crowd/Core/BP_GameState.ShowDebugByGroupAndCommand` _gamestate_ref _currentgroup "ShowDebug" false)))

(event `self.ReceiveBeginPlay`
  (set `self.bShowMouseCursor` true)
  (bind _returnvalue (`|CreateWidget` "/Game/Crowd/Core/Widget/BPW_HelperWidget.BPW_HelperWidget_C"))
  (bind _output_get (set `self.HelpMenu_ref` _returnvalue))
  (`UserWidget.AddToViewport` _output_get 0)
  (bind _asbp_game_state (cast `/Game/Crowd/Core/BP_GameState` (`GameplayStatics.GetGameState`)))
  (set `self.GameState_ref` _asbp_game_state))

(event `Key|F`
  (params (Key :type "Key Structure"))
  ;[1 0.9582 0] Input
  (:`Pressed`
    (`/Game/Crowd/Core/Widget/BPW_HelperWidget.ShowHide` (`self.HelpMenu_ref`))))

(event `Key|LeftMouseButton`
  (params (Key :type "Key Structure"))
  ;[1 0.9582 0] Input
  (:`Pressed`
    (bind _asbp_spawn_point_start (cast `/Game/Crowd/Core/AISpawn/SpawnPoint/BP_SpawnPointStart` (`self.Hit Actor`)))
    (`/Game/Crowd/Core/AISpawn/SpawnPoint/BP_SpawnPointStart.OnPressed` _asbp_spawn_point_start)))

(event `InputAction|StartCharge`
  (params (Key :type "Key Structure"))
  ;[1 0.9582 0] Input
  (:`Pressed`
    (`/Game/Crowd/Core/BP_GameState.StartCharge` (`self.GameState_ref`) (`self.CurrentGroup`))))

(event `Key|SpaceBar`
  (params (Key :type "Key Structure"))
  ;[1 0.9582 0] Input
  (:`Pressed`
    (`/Game/Crowd/Core/BP_GameState.PessedAllSpawnPoint` (`self.GameState_ref`))))

(event `CursorAction`
  (params (bIsHovered :type Boolean))
  (bind _asbp_spawn_point_start (cast `/Game/Crowd/Core/AISpawn/SpawnPoint/BP_SpawnPointStart` (`self.Hit Actor`)))
  (`/Game/Crowd/Core/AISpawn/SpawnPoint/BP_SpawnPointStart.IsOnHovered` _asbp_spawn_point_start bIsHovered))

(event `self.ReceiveTick`
  (params (DeltaSeconds :type "Float (single-precision)"))
  (bind (_bblockinghit _binitialoverlap _time _distance _location _impactpoint _normal _impactnormal _physmat _hitactor) (`GameplayStatics.BreakHitResult` (`self.GetHitResultUnderCursorByChannel` "TraceTypeQuery3")))
  (if _bblockinghit
    (`self.CursorAction` false)
    (set `self.Hit Actor` _hitactor)
    (`self.CursorAction` true)
    (else
      (`self.CursorAction` false)
      (set `self.Hit Actor` null))))

(event `InputAction|AnimBudget`
  (params (Key :type "Key Structure"))
  (bind _helpmenuab_ref (`self.HelpMenuAB_ref`))
  (:`Pressed`
    (`/Engine/EditorBlueprintResources/StandardMacros.FlipFlop`
      (:`A`
        (`/Engine/EditorBlueprintResources/StandardMacros.IsValid` (`self.HelpMenuAB_ref`)
          (:`Is Valid`
            _)
          (:`Is Not Valid`
            (bind _returnvalue (`|CreateWidget` "/Game/Crowd/Core/Widget/BPW_HElperASMenu.BPW_HelperASMenu_C"))
            (bind _output_get (set `self.HelpMenuAB_ref` _returnvalue))
            (`UserWidget.AddToViewport` _output_get 0)))
        (`Widget.SetVisibility` _helpmenuab_ref "Visible"))
      (:`B`
        (`/Engine/EditorBlueprintResources/StandardMacros.IsValid` _helpmenuab_ref
          (:`Is Valid`
            (`Widget.SetVisibility` _helpmenuab_ref "Collapsed")))))))

(event `UpdateSettingBudgetAllocator`
  (params (InParameters :type "AnimationBudgetAllocatorParameters Structure (by ref)"))
  ;[1 1 1] Anim Sharing
  (bind _output_get (set `self.In Parameters` InParameters))
  (`AnimationBudgetBlueprintLibrary.SetAnimationBudgetParameters` _output_get))

(event `Key|R`
  (params (Key :type "Key Structure"))
  ;[1 1 1] Anim Sharing
  (:`Pressed`
    (`AnimationBudgetBlueprintLibrary.EnableAnimationBudget` true)
    (`KismetSystemLibrary.ExecuteConsoleCommand` "a.Budget.Enabled 1" null)
    (`KismetSystemLibrary.ExecuteConsoleCommand` "a.Budget.Debug.Enabled 1" null)
    (`KismetSystemLibrary.ExecuteConsoleCommand` "Stat AnimationBudgetAllocator" null)))

(event `Key|T`
  (params (Key :type "Key Structure"))
  ;[1 1 1] Anim Sharing
  (:`Pressed`
    (`AnimationBudgetBlueprintLibrary.EnableAnimationBudget` false)
    (`KismetSystemLibrary.ExecuteConsoleCommand` "a.Budget.Enabled 0" null)
    (`KismetSystemLibrary.ExecuteConsoleCommand` "a.Budget.Debug.Enabled 0" null)
    (`KismetSystemLibrary.ExecuteConsoleCommand` "Stat AnimationBudgetAllocator" null)))

(event `Key|Z`
  (params (Key :type "Key Structure"))
  ;[1 1 1] crowd Detour
  (:`Pressed`
    (`KismetSystemLibrary.ExecuteConsoleCommand` "ai.crowd.DebugVisLog 1" null)
    (`KismetSystemLibrary.ExecuteConsoleCommand` "ai.crowd.DebugSelectedActors 1" null)))

(event `Key|X` :consume false
  (params (Key :type "Key Structure"))
  (bind _returnvalue (`GameplayStatics.GetPlayerController` 0))
  ;[1 1 1] crowd Detour
  (:`Pressed`
    (`KismetSystemLibrary.ExecuteConsoleCommand` "ai.crowd.DrawDebugBoundaries 1" _returnvalue)
    (`KismetSystemLibrary.ExecuteConsoleCommand` "ai.crowd.DrawDebugCollisionSegments 1" _returnvalue)
    (`KismetSystemLibrary.ExecuteConsoleCommand` "ai.crowd.DrawDebugCorners 1" _returnvalue)
    (`KismetSystemLibrary.ExecuteConsoleCommand` "ai.crowd.DrawDebugNeighbors 1" _returnvalue)
    (`KismetSystemLibrary.ExecuteConsoleCommand` "ai.crowd.DrawDebugPath 1" _returnvalue)
    (`KismetSystemLibrary.ExecuteConsoleCommand` "ai.crowd.DrawDebugPathOptimization 1" _returnvalue)
    (`KismetSystemLibrary.ExecuteConsoleCommand` "ai.crowd.DrawDebugVelocityObstacles 1" _returnvalue)))

(fn `UserConstructionScript`)